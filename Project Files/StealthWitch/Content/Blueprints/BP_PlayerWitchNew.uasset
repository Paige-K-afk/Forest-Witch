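; BP_PlayerWitchNew is the player-controlled witch character, handling movement, jumping, position reset and a victory pose.
; On BeginPlay it binds its movement, jump and reset events to CON_WitchController and saves the capsule's location as the spawn point.
; Direction events set world-axis components of CurrentVelocity, which Tick feeds to AddMovementInput.
; While HasWon is true, Tick also turns the capsule around and moves the camera to Wincam.
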(event `self.ReceiveBeginPlay`
  (bind _ascon_witch_controller (cast `/Game/Blueprints/CON_WitchController` (`GameplayStatics.GetPlayerController` 0)))
  (add `/Game/Blueprints/CON_WitchController.Forward` _ascon_witch_controller (delegate `MoveForwards`))
  (add `/Game/Blueprints/CON_WitchController.Backwards` _ascon_witch_controller (delegate `MoveBackwards`))
  (add `/Game/Blueprints/CON_WitchController.Left` _ascon_witch_controller (delegate `MoveLeft`))
  (add `/Game/Blueprints/CON_WitchController.Right` _ascon_witch_controller (delegate `MoveRight`))
  (add `/Game/Blueprints/CON_WitchController.StopForward` _ascon_witch_controller (delegate `StopForw`))
  (add `/Game/Blueprints/CON_WitchController.StopBackward` _ascon_witch_controller (delegate `StopBack`))
  (add `/Game/Blueprints/CON_WitchController.StopLeft` _ascon_witch_controller (delegate `StopLeft`))
  (add `/Game/Blueprints/CON_WitchController.StopRight` _ascon_witch_controller (delegate `StopRight`))
  (add `/Game/Blueprints/CON_WitchController.Jump` _ascon_witch_controller (delegate `playerJump`))
  (add `/Game/Blueprints/CON_WitchController.StopJump` _ascon_witch_controller (delegate `playerStopJump`))
  (add `/Game/Blueprints/CON_WitchController.Resetplayerpos` _ascon_witch_controller (delegate `resetPlayerPos`))
  (set `self.Spawn` (`SceneComponent.K2_GetComponentLocation` (`self.CapsuleComponent`))))

(event `MoveRight`
  (bind (_currentvelocity_x _currentvelocity_y _currentvelocity_z) (`KismetMathLibrary.BreakVector` (`self.CurrentVelocity`)))
  (set `self.CurrentVelocity` (`KismetMathLibrary.MakeVector` _currentvelocity_x (`self.MoveSpeed`) _currentvelocity_z)))

(event `MoveForwards`
  (bind (_currentvelocity_x _currentvelocity_y _currentvelocity_z) (`KismetMathLibrary.BreakVector` (`self.CurrentVelocity`)))
  (set `self.CurrentVelocity` (`KismetMathLibrary.MakeVector` (`self.MoveSpeed`) _currentvelocity_y _currentvelocity_z)))

(event `MoveLeft`
  (bind (_currentvelocity_x _currentvelocity_y _currentvelocity_z) (`KismetMathLibrary.BreakVector` (`self.CurrentVelocity`)))
  (set `self.CurrentVelocity` (`KismetMathLibrary.MakeVector` _currentvelocity_x (* (`self.MoveSpeed`) -1.0) _currentvelocity_z)))

(event `StopForw`
  (bind (_currentvelocity_x _currentvelocity_y _currentvelocity_z) (`KismetMathLibrary.BreakVector` (`self.CurrentVelocity`)))
  (set `self.CurrentVelocity` (`KismetMathLibrary.MakeVector` 0.0 _currentvelocity_y _currentvelocity_z) :!label _label))

(event `StopLeft`
  (bind (_currentvelocity_x _currentvelocity_y _currentvelocity_z) (`KismetMathLibrary.BreakVector` (`self.CurrentVelocity`)))
  (set `self.CurrentVelocity` (`KismetMathLibrary.MakeVector` _currentvelocity_x 0.0 _currentvelocity_z) :!label _label_2))

(event `MoveBackwards`
  (bind (_currentvelocity_x _currentvelocity_y _currentvelocity_z) (`KismetMathLibrary.BreakVector` (`self.CurrentVelocity`)))
  (set `self.CurrentVelocity` (`KismetMathLibrary.MakeVector` (* (`self.MoveSpeed`) -1.0) _currentvelocity_y _currentvelocity_z)))

(event `resetPlayerPos`
  (`self.K2_SetActorLocation` (`self.Spawn`) false true))

(event `StopBack`
  (goto _label))

(event `StopRight`
  (goto _label_2))

(event `playerJump`
  (`self.Jump`))

(event `playerStopJump`
  (`self.StopJumping`))

(event `self.ReceiveTick`
  (params (DeltaSeconds :type "Float (single-precision)"))
  (bind (_currentvelocity_x _currentvelocity_y _currentvelocity_z) (`KismetMathLibrary.BreakVector` (`self.CurrentVelocity`)))
  (bind _capsulecomponent (`self.CapsuleComponent`))
  ;[1 1 1] Updates the stored velocity and applies it to the player.
  (bind _output_get (set `self.StoredVelocuty` (`KismetMathLibrary.MakeVector` _currentvelocity_x _currentvelocity_y _currentvelocity_z)))
  (`self.AddMovementInput` _output_get)
  ;[1 0.4972 0.832] has the player won.
  (if (`self.HasWon`)
    ;[1 0.1771 0.455] This only runs when the player has won. This is a victory screen
    (`SceneComponent.K2_SetWorldLocationAndRotation` _capsulecomponent (`SceneComponent.K2_GetComponentLocation` _capsulecomponent) (struct :`Yaw` -180.0) false true)
    (`SceneComponent.K2_SetWorldLocationAndRotation` (`self.Camera`) (`self.wincam`) (struct :`Pitch` -20.0) false true)))

(fn `UserConstructionScript`)