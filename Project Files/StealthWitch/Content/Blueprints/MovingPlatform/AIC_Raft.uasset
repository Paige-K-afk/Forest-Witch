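; AI controller for the raft moving platform, running the BT_Raft behavior tree.
; BeginPlay starts the tree and writes hardcoded StartingPosition and EndingPosition vectors to the blackboard.
; Every Tick it polls RaftHasPlayer on the controlled BP_Raft and mirrors it to the HasPlayer blackboard key through two helper functions.
; The fallback cast to BP_MovingPlatformAI leads nowhere, as its player check is disconnected.
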(event `self.ReceiveBeginPlay`
  (bind _returnvalue (`AIBlueprintHelperLibrary.GetBlackboard` null))
  (`self.RunBehaviorTree` "/Game/Blueprints/MovingPlatform/BT_Raft.BT_Raft")
  (`BlackboardComponent.SetValueAsVector` _returnvalue "StartingPosition" (7651.356934 4132.0 375.0))
  (`BlackboardComponent.SetValueAsVector` _returnvalue "EndingPosition" (10341.514648 4132.0 375.0)))

(event `self.ReceiveTick`
  (params (DeltaSeconds :type "Float (single-precision)"))
  (bind _returnvalue (`self.K2_GetPawn`))
  (bind _asbp_raft (cast `/Game/Blueprints/MovingPlatform/BP_Raft` _returnvalue)
    (:`then`
      (if (`/Game/Blueprints/MovingPlatform/BP_Raft.RaftHasPlayer` _asbp_raft)
        (`self.PlayerOverlapFunc`)
        (else
          (`self.PlayerNoLongerOverlapFunc`))))
    (:`CastFailed`
      (bind _asbp_moving_platform_ai (cast `/Game/Blueprints/MovingPlatform/BP_MovingPlatformAI` _returnvalue)))))

(fn `PlayerNoLongerOverlapFunc`
  (`BlackboardComponent.SetValueAsBool` (`AIBlueprintHelperLibrary.GetBlackboard` null) "HasPlayer" false))

(fn `PlayerOverlapFunc`
  (`BlackboardComponent.SetValueAsBool` (`AIBlueprintHelperLibrary.GetBlackboard` null) "HasPlayer" true))

(fn `UserConstructionScript`)