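; BP_mrFish is an actor that launches two fish components with physics impulses while the player witch is nearby.
; Entering the ActivationZone as BP_PlayerWitchNew fires both fish immediately and sets a near-player flag, which leaving the zone clears.
; While the flag is set, Tick accumulates delta time and re-applies the Strength impulse to both fish each time TimeBetweenFish elapses.
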(event `self.ReceiveBeginPlay`)

(event `self.ReceiveTick`
  (params (DeltaSeconds :type "Float (single-precision)"))
  (bind _strength (`self.strength`))
  (bind _timesincelastfish (`self.TimeSinceLastFish`))
  (if (`self.playernearfish`)
    (if (>= _timesincelastfish (`self.TimeBetweenFish`))
      (set `self.TimeSinceLastFish` 0.0)
      (`PrimitiveComponent.AddImpulse` (`self.Fish1`) _strength "None" false)
      (`PrimitiveComponent.AddImpulse` (`self.Fish2`) _strength "None" false)
      (else
        (set `self.TimeSinceLastFish` (+ _timesincelastfish DeltaSeconds))))))

(event `self.ActivationZone.OnComponentBeginOverlap`
  (params (OverlappedComponent :type "PrimitiveComponent Object Reference") (OtherActor :type "Actor Object Reference") (OtherComp :type "PrimitiveComponent Object Reference") (OtherBodyIndex :type Integer) (bFromSweep :type Boolean) (SweepResult :type "HitResult Structure (by ref)"))
  (bind _strength (`self.strength`))
  (cast `/Game/Blueprints/BP_PlayerWitchNew` OtherActor)
  (`PrimitiveComponent.AddImpulse` (`self.Fish1`) _strength "None" false)
  (`PrimitiveComponent.AddImpulse` (`self.Fish2`) _strength "None" false)
  (set `self.playernearfish` true))

(event `self.ActivationZone.OnComponentEndOverlap`
  (params (OverlappedComponent :type "PrimitiveComponent Object Reference") (OtherActor :type "Actor Object Reference") (OtherComp :type "PrimitiveComponent Object Reference") (OtherBodyIndex :type Integer))
  (cast `/Game/Blueprints/BP_PlayerWitchNew` OtherActor)
  (set `self.playernearfish` false))

(fn `UserConstructionScript`
  (set `self.TimeSinceLastFish` 0.0)
  (set `self.playernearfish` false))