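; AI controller for the bird enemy that runs the BT_Bird behavior tree and reacts to sighting the player witch or a wolf.
; Sight updates from AI Perception write the spotted actor and a witch-or-wolf flag to the Blackboard, clearing the actor when sensing fails.
; Spotting the witch also stores her location, makes noise at the receiver's location and plays a 2D chirp.
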(event `self.ReceiveBeginPlay`
  (`self.RunBehaviorTree` "/Game/Blueprints/BirbEnemy/BT_Bird.BT_Bird"))

(event `self.AIPerception.OnTargetPerceptionUpdated`
  (params (Actor :type "Actor Object Reference") (Stimulus :type "AIStimulus Structure"))
  (bind _returnvalue (`AIPerceptionSystem.GetSenseClassForStimulus` Stimulus))
  (if (== _returnvalue "/Script/AIModule.AISense_Sight")
    (`self.SpottedSomethingFunk` Actor Stimulus)))

(fn `SpottedSomethingFunk`
  (params (Actor :type "Actor Object Reference") (Sense :type "AIStimulus Structure"))
  (bind _returnvalue (`AIBlueprintHelperLibrary.GetBlackboard` null))
  (bind _asbp_player_witch_new (cast `/Game/Blueprints/BP_PlayerWitchNew` Actor)
    (:`then`
      (if Sense_bSuccessfullySensed
        (`BlackboardComponent.SetValueAsObject` _returnvalue "spottedActor" _asbp_player_witch_new)
        (`BlackboardComponent.SetValueAsBool` _returnvalue "SpottedActorIsWitch" true)
        (`BlackboardComponent.SetValueAsVector` _returnvalue "SpottedActorLocation" Sense_StimulusLocation)
        (`self.MakeNoise` 1.0 null Sense_ReceiverLocation)
        (`GameplayStatics.PlaySound2D` "/Game/Sound/SC_Chirp.SC_Chirp" 1.0 1.0 0.0 null null)
        (else
          ;[1 1 1] If not fully sensed, unset spotted object
          (`BlackboardComponent.SetValueAsObject` _returnvalue "spottedActor" null :!label _label))))
    (:`CastFailed`
      (bind _asbp_wolf (cast `/Game/Blueprints/wolfEnemy/BP_Wolf` Actor))
      (if Sense_bSuccessfullySensed
        (`BlackboardComponent.SetValueAsObject` _returnvalue "spottedActor" _asbp_wolf)
        (`BlackboardComponent.SetValueAsBool` _returnvalue "SpottedActorIsWitch" false)
        (else
          (goto _label))))))

(fn `UserConstructionScript`)