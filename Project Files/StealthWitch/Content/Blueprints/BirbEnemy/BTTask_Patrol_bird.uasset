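; Behavior tree task that moves a BP_Bird enemy along its patrol route, one node per execution.
; It sends the bird with AIMoveTo to the PatrolNodes entry at CurrentNode, then advances the index, wrapping to zero after the last node.
; It finishes successfully on arrival, and fails if the move fails, the pawn is not a BP_Bird or the node list is empty.
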(event `self.ReceiveExecuteAI`
  (params (OwnerController :type "AIController Object Reference") (ControlledPawn :type "Pawn Object Reference"))
  (bind _asbp_bird (cast `/Game/Blueprints/BirbEnemy/BP_Bird` ControlledPawn)
    (:`then`
      (bind _patrol_nodes (`/Game/Blueprints/BirbEnemy/BP_Bird.Patrol Nodes` _asbp_bird))
      (if (> (`KismetArrayLibrary.Array_Length` _patrol_nodes) 0)
        (bind _current_node (`/Game/Blueprints/BirbEnemy/BP_Bird.Current Node` _asbp_bird))
        (`|AIMoveTo` _asbp_bird (`|GetArrayItem` _patrol_nodes _current_node) null
          (:`OnSuccess`
            (bind _returnvalue (+ _current_node 1))
            (if (== (`KismetArrayLibrary.Array_Length` _patrol_nodes) _returnvalue)
              (set `/Game/Blueprints/BirbEnemy/BP_Bird.Current Node` 0 _asbp_bird)
              (else
                (set `/Game/Blueprints/BirbEnemy/BP_Bird.Current Node` _returnvalue _asbp_bird)))
            (`self.FinishExecute` true))
          (:`OnFail`
            ;[1 1 1] Fails go here
            (`self.FinishExecute` false :!label _label)))
        (else
          (goto _label))))
    (:`CastFailed`
      (goto _label))))