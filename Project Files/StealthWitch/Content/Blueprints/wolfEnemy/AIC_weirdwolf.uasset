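; AI controller for the weird wolf enemy that runs its behavior tree and feeds it perception results.
; Sight of the player witch sets the spotted actor, plays a roar and clears any heard actor; losing sight stores the last seen location.
; Hearing a bird sets or clears the heard actor and records the stimulus location in the same last-spotted location key.
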(event `self.AIPerception.OnTargetPerceptionUpdated`
  (params (Actor :type "Actor Object Reference") (Stimulus :type "AIStimulus Structure"))
  (bind _returnvalue (`AIPerceptionSystem.GetSenseClassForStimulus` Stimulus))
  (if (== _returnvalue "/Script/AIModule.AISense_Sight")
    (`self.SpottedPlayerFunk` Actor Stimulus))
  (if (== _returnvalue "/Script/AIModule.AISense_Hearing")
    (`self.HeardBirdFunk` Actor Stimulus)))

(event `self.ReceiveBeginPlay`
  (`self.RunBehaviorTree` "/Game/Blueprints/wolfEnemy/BT_WeirdWolf.BT_WeirdWolf"))

(fn `HeardBirdFunk`
  (params (SpottedItem :type "Actor Object Reference") (Sense :type "AIStimulus Structure"))
  (bind _returnvalue (`AIBlueprintHelperLibrary.GetBlackboard` null))
  (bind _asbp_bird (cast `/Game/Blueprints/BirbEnemy/BP_Bird` SpottedItem))
  (if Sense_bSuccessfullySensed
    (`BlackboardComponent.SetValueAsObject` _returnvalue "HeardActor" _asbp_bird)
    (`BlackboardComponent.SetValueAsVector` _returnvalue "lastSpottedLocation" Sense_StimulusLocation)
    (else
      (`BlackboardComponent.SetValueAsObject` _returnvalue "HeardActor" null)
      (`BlackboardComponent.SetValueAsVector` _returnvalue "lastSpottedLocation" Sense_StimulusLocation))))

(fn `SpottedPlayerFunk`
  (params (SpottedItem :type "Actor Object Reference") (Sense :type "AIStimulus Structure"))
  (bind _returnvalue (`AIBlueprintHelperLibrary.GetBlackboard` null))
  (bind _asbp_player_witch_new (cast `/Game/Blueprints/BP_PlayerWitchNew` SpottedItem))
  (if Sense_bSuccessfullySensed
    (`BlackboardComponent.SetValueAsObject` _returnvalue "spottedActor" _asbp_player_witch_new)
    (`GameplayStatics.PlaySound2D` "/Game/Sound/SC_roar.SC_roar" 1.0 1.0 0.0 null null)
    ;[1 1 1] wolf is no longer hearing if player is in sught
    (`BlackboardComponent.SetValueAsObject` _returnvalue "HeardActor" null)
    (else
      (`BlackboardComponent.SetValueAsObject` _returnvalue "spottedActor" null)
      (`BlackboardComponent.SetValueAsVector` _returnvalue "lastSpottedLocation" Sense_StimulusLocation))))

(fn `UserConstructionScript`)