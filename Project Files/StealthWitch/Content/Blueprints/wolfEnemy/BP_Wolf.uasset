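; BP_Wolf is a wolf enemy whose DeathCube volume costs the player witch a life and teleports them to Spawn on contact.
; A CanOverlapPlayer flag blocks repeat hits until the overlap ends.
; When lives run out, Playerdead makes Tick add a BP_Die widget every frame while a timer runs, then load the main menu.
; The file contains no movement or AI logic.
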(event `self.DeathCube.OnComponentEndOverlap`
  (params (OverlappedComponent :type "PrimitiveComponent Object Reference") (OtherActor :type "Actor Object Reference") (OtherComp :type "PrimitiveComponent Object Reference") (OtherBodyIndex :type Integer))
  (cast `/Game/Blueprints/BP_PlayerWitchNew` OtherActor)
  (if (not (`self.canOverlapPlayer`))
    (set `self.canOverlapPlayer` true)))

(event `self.DeathCube.OnComponentBeginOverlap`
  (params (OverlappedComponent :type "PrimitiveComponent Object Reference") (OtherActor :type "Actor Object Reference") (OtherComp :type "PrimitiveComponent Object Reference") (OtherBodyIndex :type Integer) (bFromSweep :type Boolean) (SweepResult :type "HitResult Structure (by ref)"))
  (bind _asbp_player_witch_new (cast `/Game/Blueprints/BP_PlayerWitchNew` OtherActor))
  (if (`self.canOverlapPlayer`)
    ;[1 1 1] Soft death: reset.
    (`self.K2_SetActorLocation` _asbp_player_witch_new (`self.Spawn`) false true)
    (bind _output_get (set `/Game/Blueprints/BP_PlayerWitchNew.Lives` (- (`/Game/Blueprints/BP_PlayerWitchNew.Lives` _asbp_player_witch_new) 1) _asbp_player_witch_new))
    (if (<= _output_get 0)
      (set `self.playerdead` true)
      (else
        (set `self.canOverlapPlayer` false)))))

(event `self.ReceiveBeginPlay`
  (set `self.playerdead` false)
  (set `self.canOverlapPlayer` true))

(event `self.ReceiveTick`
  (params (DeltaSeconds :type "Float (single-precision)"))
  (bind _deathtime (`self.DeathTime`))
  (if (`self.playerdead`)
    (bind _returnvalue (`|CreateWidget` "/Game/Blueprints/wolfEnemy/BP_Die.BP_Die_C"))
    (`UserWidget.AddToViewport` _returnvalue 0)
    (if (>= _deathtime (`self.GameOverScreenDuration`))
      (`GameplayStatics.OpenLevel` "L_MainMenu")
      (else
        (set `self.DeathTime` (+ _deathtime DeltaSeconds))))))

(fn `UserConstructionScript`)