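; Behavior tree task that walks a BP_Wolf enemy to the next point in its patrol route.
; It moves the controlled wolf to the PatrolNodes entry at CurrentNode, then advances the index, wrapping to zero after the last node.
; The task succeeds after a completed move and fails if the pawn is not a wolf, has no nodes, or the move fails.
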(event `self.ReceiveExecuteAI`
  (params (OwnerController :type "AIController Object Reference") (ControlledPawn :type "Pawn Object Reference"))
  (bind _asbp_wolf (cast `/Game/Blueprints/wolfEnemy/BP_Wolf` ControlledPawn)
    (:`then`
      (bind _patrol_nodes (`/Game/Blueprints/wolfEnemy/BP_Wolf.Patrol Nodes` _asbp_wolf))
      (if (> (`KismetArrayLibrary.Array_Length` _patrol_nodes) 0)
        (bind _current_node (`/Game/Blueprints/wolfEnemy/BP_Wolf.Current Node` _asbp_wolf))
        (`|AIMoveTo` _asbp_wolf (`|GetArrayItem` _patrol_nodes _current_node) null
          (:`OnSuccess`
            (bind _returnvalue (+ _current_node 1))
            (if (== (`KismetArrayLibrary.Array_Length` _patrol_nodes) _returnvalue)
              (set `/Game/Blueprints/wolfEnemy/BP_Wolf.Current Node` 0 _asbp_wolf)
              (else
                (set `/Game/Blueprints/wolfEnemy/BP_Wolf.Current Node` _returnvalue _asbp_wolf)))
            (`self.FinishExecute` true))
          (:`OnFail`
            ;[1 1 1] Fails go here
            (`self.FinishExecute` false :!label _label)))
        (else
          (goto _label))))
    (:`CastFailed`
      (goto _label))))