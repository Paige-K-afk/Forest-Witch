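; Player controller for the witch character that turns keyboard input into event dispatcher calls.
; W, A, S, D and Space each call a start dispatcher on press and a stop dispatcher on release for movement and jumping.
; Escape and L both call the reset player position dispatcher.
; The controller holds no movement logic itself, leaving the response to whatever binds to those dispatchers.
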(event `Key|W`
  (params (Key :type "Key Structure"))
  (:`Pressed`
    (`self.Forward`))
  (:`Released`
    (`self.StopForward`)))

(event `Key|A`
  (params (Key :type "Key Structure"))
  (:`Pressed`
    (`self.Left`))
  (:`Released`
    (`self.StopLeft`)))

(event `Key|S`
  (params (Key :type "Key Structure"))
  (:`Pressed`
    (`self.Backwards`))
  (:`Released`
    (`self.StopBackward`)))

(event `Key|D`
  (params (Key :type "Key Structure"))
  (:`Pressed`
    (`self.Right`))
  (:`Released`
    (`self.StopRight`)))

(event `Key|SpaceBar`
  (params (Key :type "Key Structure"))
  (:`Pressed`
    (`self.Jump`))
  (:`Released`
    (`self.StopJump`)))

(event `Key|Escape`
  (params (Key :type "Key Structure"))
  (:`Pressed`
    (`self.Resetplayerpos` :!label _label)))

(event `Key|L`
  (params (Key :type "Key Structure"))
  (:`Pressed`
    (goto _label)))

(fn `UserConstructionScript`)